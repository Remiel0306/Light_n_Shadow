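; Enemy shadow actor that casts up to three query-only shadow colliders away from nearby BP_LightBall actors and reports whether it links to other shadows.
; Capsule overlaps assign balls to three slots and reset a slot's collider on exit.
; Each Tick, a line trace from Top, opposite each ball, aims and stretches that slot's box collider.
; Overlaps with tagged enemies, objects or their shadows toggle ConnectOBJ, exposed through IsShadowLinkActive.
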(event OnComponentBeginOverlap(CapsuleComponent)
  (params (OverlappedComponent :type Primitive%20Component%20Object%20Reference) (OtherActor :type Actor%20Object%20Reference) (OtherComp :type Primitive%20Component%20Object%20Reference) (OtherBodyIndex :type Integer) (bFromSweep :type Boolean) (SweepResult :type Hit%20Result%20Structure%20%28by%20ref%29))
  (if (Components|ComponentHasTag OtherComp "Object Shadow")
    (Variables|Default|SetConnect%20OBJ true :!label _label)
    (elif (Actor|ActorHasTag OtherActor "Object")
      (goto _label)
      (else
        _)))
  (bind _asbp_light_ball (Utilities|Casting|CastToBP_LightBall OtherActor))
  (Utilities|Array|Add (Variables|Default|GetActive%20Ball) _asbp_light_ball)
  (Variables|Default|SetisInChecker true)
  (if (Utilities|IsValid (Utilities|Array|Get(acopy) (Variables|Default|GetSlot%20Owners)))
    (if (Utilities|IsValid (Utilities|Array|Get(acopy) (Variables|Default|GetSlot%20Owners) 1))
      (if (not (Utilities|IsValid (Utilities|Array|Get(acopy) (Variables|Default|GetSlot%20Owners) 2)))
        (Utilities|Array|SetArrayElem (Variables|Default|GetSlot%20Owners) 2 OtherActor))
      (else
        (Utilities|Array|SetArrayElem (Variables|Default|GetSlot%20Owners) 1 OtherActor)))
    (else
      (Utilities|Array|SetArrayElem (Variables|Default|GetSlot%20Owners) 0 OtherActor))))

(event OnComponentEndOverlap(CapsuleComponent)
  (params (OverlappedComponent :type Primitive%20Component%20Object%20Reference) (OtherActor :type Actor%20Object%20Reference) (OtherComp :type Primitive%20Component%20Object%20Reference) (OtherBodyIndex :type Integer))
  (if (Components|ComponentHasTag OtherComp "Object Shadow")
    (Variables|Default|SetConnect%20OBJ false :!label _label)
    (elif (Actor|ActorHasTag OtherActor "Object")
      (goto _label)
      (else
        _)))
  (Utilities|Array|Clear (Variables|Default|GetActive%20Ball))
  (for _index (range 0 2)
    (if (== (Utilities|Array|Get(acopy) (Variables|Default|GetSlot%20Owners) _index) OtherActor)
      (Variables|Default|SetisInChecker false)
      (CallFunction|ResetOneShadowCollider (Utilities|Select :Index _index :Option%200 (Variables|Default|GetShaodwColliderRoot1) :Option%201 (Variables|Default|GetShaodwColliderRoot2) :Option%202 (Variables|Default|GetShaodwColliderRoot3)) (Utilities|Select :Index _index :Option%200 (Variables|Default|GetShadowCollider1) :Option%201 (Variables|Default|GetShadowCollider2) :Option%202 (Variables|Default|GetShadowCollider3)))
      (Utilities|Array|SetArrayElem (Variables|Default|GetSlot%20Owners) _index 0)
      (for _index_2 (range 0 0)
        _))))

(event OnComponentBeginOverlap(ShadowCollider3)
  (params (OverlappedComponent :type Primitive%20Component%20Object%20Reference) (OtherActor :type Actor%20Object%20Reference) (OtherComp :type Primitive%20Component%20Object%20Reference) (OtherBodyIndex :type Integer) (bFromSweep :type Boolean) (SweepResult :type Hit%20Result%20Structure%20%28by%20ref%29))
  (if (Math|Boolean|ORBoolean (Components|ComponentHasTag OtherComp "Enemy Shadow") (Actor|ActorHasTag OtherActor "Enemy") (Components|ComponentHasTag OtherComp "Object Shadow") (Actor|ActorHasTag OtherActor "Object"))
    (Variables|Default|SetConnect%20OBJ true)))

(event OnComponentBeginOverlap(ShadowCollider2)
  (params (OverlappedComponent :type Primitive%20Component%20Object%20Reference) (OtherActor :type Actor%20Object%20Reference) (OtherComp :type Primitive%20Component%20Object%20Reference) (OtherBodyIndex :type Integer) (bFromSweep :type Boolean) (SweepResult :type Hit%20Result%20Structure%20%28by%20ref%29))
  (if (Math|Boolean|ORBoolean (Components|ComponentHasTag OtherComp "Enemy Shadow") (Actor|ActorHasTag OtherActor "Enemy") (Components|ComponentHasTag OtherComp "Object Shadow") (Actor|ActorHasTag OtherActor "Object"))
    (Variables|Default|SetConnect%20OBJ true)))

(event OnComponentBeginOverlap(ShadowCollider1)
  (params (OverlappedComponent :type Primitive%20Component%20Object%20Reference) (OtherActor :type Actor%20Object%20Reference) (OtherComp :type Primitive%20Component%20Object%20Reference) (OtherBodyIndex :type Integer) (bFromSweep :type Boolean) (SweepResult :type Hit%20Result%20Structure%20%28by%20ref%29))
  (if (Math|Boolean|ORBoolean (Components|ComponentHasTag OtherComp "Enemy Shadow") (Actor|ActorHasTag OtherActor "Enemy") (Components|ComponentHasTag OtherComp "Object Shadow") (Actor|ActorHasTag OtherActor "Object"))
    (Variables|Default|SetConnect%20OBJ true)))

(event OnComponentEndOverlap(ShadowCollider1)
  (params (OverlappedComponent :type Primitive%20Component%20Object%20Reference) (OtherActor :type Actor%20Object%20Reference) (OtherComp :type Primitive%20Component%20Object%20Reference) (OtherBodyIndex :type Integer))
  (if (Math|Boolean|ORBoolean (Components|ComponentHasTag OtherComp "Enemy Shadow") (Actor|ActorHasTag OtherActor "Enemy") (Components|ComponentHasTag OtherComp "Object Shadow") (Actor|ActorHasTag OtherActor "Object"))
    (Variables|Default|SetConnect%20OBJ false)))

(event OnComponentEndOverlap(ShadowCollider2)
  (params (OverlappedComponent :type Primitive%20Component%20Object%20Reference) (OtherActor :type Actor%20Object%20Reference) (OtherComp :type Primitive%20Component%20Object%20Reference) (OtherBodyIndex :type Integer))
  (if (Math|Boolean|ORBoolean (Components|ComponentHasTag OtherComp "Enemy Shadow") (Actor|ActorHasTag OtherActor "Enemy") (Components|ComponentHasTag OtherComp "Object Shadow") (Actor|ActorHasTag OtherActor "Object"))
    (Variables|Default|SetConnect%20OBJ false)))

(event OnComponentEndOverlap(ShadowCollider3)
  (params (OverlappedComponent :type Primitive%20Component%20Object%20Reference) (OtherActor :type Actor%20Object%20Reference) (OtherComp :type Primitive%20Component%20Object%20Reference) (OtherBodyIndex :type Integer))
  (if (Math|Boolean|ORBoolean (Components|ComponentHasTag OtherComp "Enemy Shadow") (Actor|ActorHasTag OtherActor "Enemy") (Components|ComponentHasTag OtherComp "Object Shadow") (Actor|ActorHasTag OtherActor "Object"))
    (Variables|Default|SetConnect%20OBJ false)))

(event Custom|Enemy%20Die
  (Development|PrintString "Enemy die")
  (Actor|DestroyActor))

(event Custom|Shadow%20Collision%202
  (params (Ball :type Actor%20Object%20Reference))
  (bind _shadowcollider2 (Variables|Default|GetShadowCollider2))
  (CallFunction|ShadowCollisionCompute Ball (Variables|Default|GetShaodwColliderRoot2) _shadowcollider2)
  (Collision|SetCollisionEnabled _shadowcollider2 "QueryOnly"))

(event Custom|Shadow%20Collision%201
  (params (Ball :type Actor%20Object%20Reference))
  (bind _shadowcollider1 (Variables|Default|GetShadowCollider1))
  (CallFunction|ShadowCollisionCompute Ball (Variables|Default|GetShaodwColliderRoot1) _shadowcollider1)
  (Collision|SetCollisionEnabled _shadowcollider1 "QueryOnly"))

(event Custom|Shadow%20Collision%20Compute
  (params (Ball :type Actor%20Object%20Reference) (Target%20Root :type Scene%20Component%20Object%20Reference) (Target%20Collider :type Box%20Component%20Object%20Reference))
  (bind _returnvalue (Transformation|GetActorLocation Ball))
  (bind _top (Variables|Default|GetTop))
  (bind _returnvalue_2 (Transformation|GetWorldLocation _top))
  (bind _returnvalue_3 (- _returnvalue_2 _returnvalue))
  (bind _returnvalue_4 (Math|Vector|Normalize _returnvalue_3))
  (bind _returnvalue_5 (* _returnvalue_4 6e+02))
  (bind _returnvalue_6 (+ _returnvalue_2 _returnvalue_5))
  (bind (_outhit _returnvalue_7) (Collision|LineTraceByChannel _returnvalue_2 _returnvalue_6 "TraceTypeQuery1" false 0 "ForDuration"))
  (bind _output_get (Variables|Default|SetShadow%20farthest%20location (Math|Vector|SelectVector (.Location (Collision|BreakHitResult _outhit)) (+ _returnvalue_2 (* (- _returnvalue_6 _returnvalue_2) 0.6)) _returnvalue_7)))
  (Variables|Default|SetShadow%20colision%20distance (Math|Vector|VectorLength (- _output_get (Transformation|GetWorldLocation Target%20Root))))
  (Transformation|SetWorldRotation Target%20Root (Math|Rotator|FindLookatRotation (Transformation|GetWorldLocation (Variables|Default|GetTop)) (Variables|Default|GetShadow%20farthest%20location)) false false)
  (Components|Box|SetBoxExtent Target%20Collider (Math|Vector|MakeVector 8e+01 (/ (Math|Vector|VectorLength (- _output_get (Transformation|GetWorldLocation Target%20Root))) 2.5) 5e+01) true)
  (Transformation|SetRelativeLocation Target%20Collider (Math|Vector|MakeVector (/ (Math|Vector|VectorLength (- _output_get (Transformation|GetWorldLocation Target%20Root))) 2.5) 0.0 0.0) false false))

(event Custom|Check%20Overlapping%20Light%20Checker
  (for _array_element (Collision|GetOverlappingActors (Variables|Collision|GetCapsuleComponent) "/Game/BluePrint/BP_LightBall.BP_LightBall_C" :!class /Script/Engine.PrimitiveComponent)
    (if (== (Utilities|Array|Get(acopy) (Variables|Default|GetSlot%20Owners)) _array_element)
      (CallFunction|ShadowCollision1 _array_element)
      (elif (== (Utilities|Array|Get(acopy) (Variables|Default|GetSlot%20Owners) 1) _array_element)
        (CallFunction|ShadowCollision2 _array_element)
        (elif (== (Utilities|Array|Get(acopy) (Variables|Default|GetSlot%20Owners) 2) _array_element)
          (CallFunction|ShadowCollision3 _array_element))))))

(event Custom|Shadow%20Collision%203
  (params (Ball :type Actor%20Object%20Reference))
  (bind _shadowcollider3 (Variables|Default|GetShadowCollider3))
  (CallFunction|ShadowCollisionCompute Ball (Variables|Default|GetShaodwColliderRoot3) _shadowcollider3)
  (Collision|SetCollisionEnabled _shadowcollider3 "QueryOnly"))

(event EventBeginPlay
  (Collision|SetCollisionEnabled (Variables|Default|GetShadowCollider2) "NoCollision")
  (Utilities|Array|Clear (Variables|Default|GetSlot%20Owners))
  (Utilities|Array|Add (Variables|Default|GetSlot%20Owners) 0)
  (Utilities|Array|Add (Variables|Default|GetSlot%20Owners) 0)
  (Utilities|Array|Add (Variables|Default|GetSlot%20Owners) 0))

(event Collision|EventActorBeginOverlap
  (params (OtherActor :type Actor%20Object%20Reference)))

(event EventTick
  (params (DeltaSeconds :type Float%20%28single-precision%29))
  (CallFunction|CheckOverlappingLightChecker)
  (if (Variables|Default|GetConnect%20OBJ)
    _))

(fn ConstructionScript)

(fn UpdateOneShadowCollider
  (params (TargetRoot :type Scene%20Component%20Object%20Reference) (TargetCollider :type Box%20Component%20Object%20Reference) (Start :type Vector) (Dir :type Vector) (MaxDistance :type Float%20%28double-precision%29) (WidthX :type Float%20%28double-precision%29) (ThicknessZ :type Float%20%28double-precision%29))
  (bind _returnvalue (Math|Vector|Normalize Dir))
  (bind _returnvalue_2 (* _returnvalue MaxDistance))
  (bind _returnvalue_3 (+ Start _returnvalue_2))
  (bind (_outhit _returnvalue_4) (Collision|LineTraceByChannel Start _returnvalue_3 "TraceTypeQuery1" false 0 "None"))
  (Transformation|SetWorldLocation TargetRoot Start false false)
  (Transformation|SetWorldRotation TargetRoot (Math|Rotator|FindLookatRotation Start (Math|Vector|SelectVector (.Location (Collision|BreakHitResult _outhit)) _returnvalue_3 _returnvalue_4)) false false)
  (Transformation|SetRelativeLocation TargetCollider (Math|Vector|MakeVector (/ (Math|Vector|VectorLength (- (Math|Vector|SelectVector (.Location (Collision|BreakHitResult _outhit)) _returnvalue_3 _returnvalue_4) Start)) 2.5) 0.0 -4e+01) false false)
  (Components|Box|SetBoxExtent TargetCollider (Math|Vector|MakeVector WidthX (/ (Math|Vector|VectorLength (- (Math|Vector|SelectVector (.Location (Collision|BreakHitResult _outhit)) _returnvalue_3 _returnvalue_4) Start)) 2.5) ThicknessZ) true)
  (return _returnvalue_4))

(fn ResetOneShadowCollider
  (params (TargetRoot :type Scene%20Component%20Object%20Reference) (TargetCollider :type Box%20Component%20Object%20Reference))
  (Components|Box|SetBoxExtent TargetCollider (Variables|Default|GetOrigin%20colision%20size) true)
  (Collision|SetCollisionEnabled TargetCollider "NoCollision")
  (Transformation|SetRelativeLocation TargetCollider "0, 0, 0" false false)
  (Transformation|SetWorldRotation TargetRoot "0, 0, 0" false false))

(fn GetShadowOwner
  (return self))

(fn GetShadowRole
  (return (Utilities|Enum|LiteralenumE_ShadowRole "NewEnumerator2")))

(fn IsShadowLinkActive
  (return (Variables|Default|GetConnect%20OBJ)))