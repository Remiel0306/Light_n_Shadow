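; Enemy Blueprint that casts a collidable shadow box away from any BP_LightBall overlapping its capsule.
; Each Tick it traces from Top away from each overlapping ball, then rotates and stretches one shared ShadowCollider1 toward the hit or fallback point.
; Ending any capsule overlap clears ActiveBall, resets the box and disables its collision.
; UpdateOneShadowCollider generalizes the trace-and-fit step but is never called in these graphs.
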(event OnComponentBeginOverlap(CapsuleComponent)
  (params (OverlappedComponent :type Primitive%20Component%20Object%20Reference) (OtherActor :type Actor%20Object%20Reference) (OtherComp :type Primitive%20Component%20Object%20Reference) (OtherBodyIndex :type Integer) (bFromSweep :type Boolean) (SweepResult :type Hit%20Result%20Structure%20%28by%20ref%29))
  (bind _asbp_light_ball (Utilities|Casting|CastToBP_LightBall OtherActor))
  (Utilities|Array|Add (Variables|Default|GetActive%20Ball) _asbp_light_ball)
  (Variables|Default|SetisInChecker true))

(event OnComponentEndOverlap(CapsuleComponent)
  (params (OverlappedComponent :type Primitive%20Component%20Object%20Reference) (OtherActor :type Actor%20Object%20Reference) (OtherComp :type Primitive%20Component%20Object%20Reference) (OtherBodyIndex :type Integer))
  (bind _shadowcollider1 (Variables|Default|GetShadowCollider1))
  (Utilities|Array|Clear (Variables|Default|GetActive%20Ball))
  (Components|Box|SetBoxExtent _shadowcollider1 (Variables|Default|GetOrigin%20colision%20size) true)
  (Transformation|SetRelativeLocation _shadowcollider1 (Variables|Default|GetRoot%20Location) false false)
  (Transformation|SetRelativeRotation _shadowcollider1 (Math|Rotator|MakeRotator 0.0 0.0 -9e+01) false false)
  (Collision|SetCollisionEnabled (Variables|Default|GetShadowCollider1) "NoCollision"))

(event Custom|Shadow%20Collision%20Change
  (bind _shadowcollider1 (Variables|Default|GetShadowCollider1))
  (bind _top (Variables|Default|GetTop))
  (bind _returnvalue (Transformation|GetWorldLocation _top))
  ;[0.15 0.15 0.15 0.5] Coulate the colider size and rotation
  (bind (_outhit _returnvalue_2) (Collision|LineTraceByChannel _returnvalue (+ _returnvalue (* (Math|Vector|Normalize (- _returnvalue (Transformation|GetActorLocation (stale Custom|Check%20Overlapping%20Light%20Checker _array_element)))) 6e+02)) "TraceTypeQuery1" false 0 "ForDuration"))
  (bind _output_get (Variables|Default|SetShadow%20farthest%20location (Math|Vector|SelectVector (.Location (Collision|BreakHitResult _outhit)) (+ _returnvalue (* (- (+ _returnvalue (* (Math|Vector|Normalize (- _returnvalue (Transformation|GetActorLocation (stale Custom|Check%20Overlapping%20Light%20Checker _array_element)))) 6e+02)) _returnvalue) 0.6)) _returnvalue_2)))
  ;;[0.15 0.15 0.15 0.5] Set Collider size and rotation
  (Variables|Default|SetShadow%20colision%20distance (Math|Vector|VectorLength (- _output_get (Transformation|GetWorldLocation (Variables|Default|GetShaodwColliderRoot1)))))
  (Transformation|SetWorldRotation (Variables|Default|GetShaodwColliderRoot1) (Math|Rotator|FindLookatRotation (Transformation|GetWorldLocation (Variables|Default|GetTop)) (Variables|Default|GetShadow%20farthest%20location)) false false)
  (Components|Box|SetBoxExtent _shadowcollider1 (Math|Vector|MakeVector 8e+01 (/ (Math|Vector|VectorLength (- _output_get (Transformation|GetWorldLocation (Variables|Default|GetShaodwColliderRoot1)))) 2.5) 25.0) true)
  (Transformation|SetRelativeLocation _shadowcollider1 (Math|Vector|MakeVector (/ (Math|Vector|VectorLength (- _output_get (Transformation|GetWorldLocation (Variables|Default|GetShaodwColliderRoot1)))) 2.5) 0.0 0.0) false false)
  (Collision|SetCollisionEnabled (Variables|Default|GetShadowCollider1) "QueryOnly"))

(event Custom|Check%20Overlapping%20Light%20Checker
  ;[0.15 0.15 0.15 0.5] Coulate the colider size and rotation
  (for _array_element (Collision|GetOverlappingActors (Variables|Collision|GetCapsuleComponent) "/Game/BluePrint/BP_LightBall.BP_LightBall_C" :!class /Script/Engine.PrimitiveComponent)
    (CallFunction|ShadowCollisionChange)))

(event EventBeginPlay
  (Collision|SetCollisionEnabled (Variables|Default|GetShadowCollider1) "NoCollision"))

(event Collision|EventActorBeginOverlap
  (params (OtherActor :type Actor%20Object%20Reference)))

(event EventTick
  (params (DeltaSeconds :type Float%20%28single-precision%29))
  (CallFunction|CheckOverlappingLightChecker))

(fn ConstructionScript)

(fn UpdateOneShadowCollider
  (params (TargetRoot :type Scene%20Component%20Object%20Reference) (TargetCollider :type Box%20Component%20Object%20Reference) (Start :type Vector) (Dir :type Vector) (MaxDistance :type Float%20%28double-precision%29) (WidthX :type Float%20%28double-precision%29) (ThicknessZ :type Float%20%28double-precision%29))
  (bind _returnvalue (Math|Vector|Normalize Dir))
  (bind _returnvalue_2 (* _returnvalue MaxDistance))
  (bind _returnvalue_3 (+ Start _returnvalue_2))
  (bind (_outhit _returnvalue_4) (Collision|LineTraceByChannel Start _returnvalue_3 "TraceTypeQuery1" false 0 "None"))
  (Transformation|SetWorldLocation TargetRoot Start false false)
  (Transformation|SetWorldRotation TargetRoot (Math|Rotator|FindLookatRotation Start (Math|Vector|SelectVector (.Location (Collision|BreakHitResult _outhit)) _returnvalue_3 _returnvalue_4)) false false)
  (Transformation|SetRelativeLocation TargetCollider (Math|Vector|MakeVector 0.0 (/ (Math|Vector|VectorLength (- (Math|Vector|SelectVector (.Location (Collision|BreakHitResult _outhit)) _returnvalue_3 _returnvalue_4) Start)) 2.0) 0.0) false false)
  (Components|Box|SetBoxExtent TargetCollider (Math|Vector|MakeVector WidthX (/ (Math|Vector|VectorLength (- (Math|Vector|SelectVector (.Location (Collision|BreakHitResult _outhit)) _returnvalue_3 _returnvalue_4) Start)) 2.0) ThicknessZ) true)
  (return _returnvalue_4))