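; Gives an object dynamic shadow hitboxes cast away from nearby BP_LightBall actors, and tracks whether its shadow links with enemy or object shadows.
; Light balls entering the Cylinder claim one of three slots, each driving its own collider.
; On Tick, a collider is aimed along a trace away from its light, or reset when traces to both Top and Bottom are blocked.
; Tagged overlaps set the link flag, exposed with owner and role getters.
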(event OnComponentBeginOverlap(ShadowCollider1)
  (params (OverlappedComponent :type Primitive%20Component%20Object%20Reference) (OtherActor :type Actor%20Object%20Reference) (OtherComp :type Primitive%20Component%20Object%20Reference) (OtherBodyIndex :type Integer) (bFromSweep :type Boolean) (SweepResult :type Hit%20Result%20Structure%20%28by%20ref%29))
  (if (Math|Boolean|ORBoolean (Components|ComponentHasTag OtherComp "Enemy Shadow") (Actor|ActorHasTag OtherActor "Enemy") (Components|ComponentHasTag OtherComp "Object Shadow") (Actor|ActorHasTag OtherActor "Object"))
    (Variables|Default|SetConnect%20Enemy true)))

(event OnComponentBeginOverlap(Cylinder)
  (params (OverlappedComponent :type Primitive%20Component%20Object%20Reference) (OtherActor :type Actor%20Object%20Reference) (OtherComp :type Primitive%20Component%20Object%20Reference) (OtherBodyIndex :type Integer) (bFromSweep :type Boolean) (SweepResult :type Hit%20Result%20Structure%20%28by%20ref%29))
  (if (Components|ComponentHasTag OtherComp "Enemy Shadow")
    (Variables|Default|SetConnect%20Enemy true))
  (bind _asbp_light_ball (Utilities|Casting|CastToBP_LightBall OtherActor))
  (Utilities|Array|Add (Variables|Default|GetActive%20Ball) _asbp_light_ball)
  (Variables|Default|SetisInChecker true)
  (if (Utilities|IsValid (Utilities|Array|Get(acopy) (Variables|Default|GetSlot%20Onwers)))
    (if (Utilities|IsValid (Utilities|Array|Get(acopy) (Variables|Default|GetSlot%20Onwers) 1))
      (if (not (Utilities|IsValid (Utilities|Array|Get(acopy) (Variables|Default|GetSlot%20Onwers) 2)))
        (Utilities|Array|SetArrayElem (Variables|Default|GetSlot%20Onwers) 2 OtherActor))
      (else
        (Utilities|Array|SetArrayElem (Variables|Default|GetSlot%20Onwers) 1 OtherActor)))
    (else
      (Utilities|Array|SetArrayElem (Variables|Default|GetSlot%20Onwers) 0 OtherActor))))

(event OnComponentEndOverlap(Cylinder)
  (params (OverlappedComponent :type Primitive%20Component%20Object%20Reference) (OtherActor :type Actor%20Object%20Reference) (OtherComp :type Primitive%20Component%20Object%20Reference) (OtherBodyIndex :type Integer))
  (if (Components|ComponentHasTag OtherComp "Enemy Shadow")
    (Variables|Default|SetConnect%20Enemy false))
  (Utilities|Array|Clear (Variables|Default|GetActive%20Ball))
  (for _index (range 0 2)
    (if (== (Utilities|Array|Get(acopy) (Variables|Default|GetSlot%20Onwers) _index) OtherActor)
      (Variables|Default|SetisInChecker false)
      (CallFunction|ResetOneShadowCollider (Utilities|Select :Index _index :Option%200 (Variables|Default|GetShadowColliderRoot%201) :Option%201 (Variables|Default|GetShadowColliderRoot%202) :Option%202 (Variables|Default|GetShadowColliderRoot%203)) (Utilities|Select :Index _index :Option%200 (Variables|Default|GetShadow%20Collider%201) :Option%201 (Variables|Default|GetShadow%20Collider%202) :Option%202 (Variables|Default|GetShadow%20Collider%203)))
      (Utilities|Array|SetArrayElem (Variables|Default|GetSlot%20Onwers) _index 0)
      (for _index_2 (range 0 0)
        _))))

(event OnComponentBeginOverlap(ShadowCollider3)
  (params (OverlappedComponent :type Primitive%20Component%20Object%20Reference) (OtherActor :type Actor%20Object%20Reference) (OtherComp :type Primitive%20Component%20Object%20Reference) (OtherBodyIndex :type Integer) (bFromSweep :type Boolean) (SweepResult :type Hit%20Result%20Structure%20%28by%20ref%29))
  (if (Math|Boolean|ORBoolean (Components|ComponentHasTag OtherComp "Enemy Shadow") (Actor|ActorHasTag OtherActor "Enemy") (Components|ComponentHasTag OtherComp "Object Shadow") (Actor|ActorHasTag OtherActor "Object"))
    (Variables|Default|SetConnect%20Enemy true)))

(event OnComponentBeginOverlap(ShadowCollider2)
  (params (OverlappedComponent :type Primitive%20Component%20Object%20Reference) (OtherActor :type Actor%20Object%20Reference) (OtherComp :type Primitive%20Component%20Object%20Reference) (OtherBodyIndex :type Integer) (bFromSweep :type Boolean) (SweepResult :type Hit%20Result%20Structure%20%28by%20ref%29))
  (if (Math|Boolean|ORBoolean (Components|ComponentHasTag OtherComp "Enemy Shadow") (Actor|ActorHasTag OtherActor "Enemy") (Components|ComponentHasTag OtherComp "Object Shadow") (Actor|ActorHasTag OtherActor "Object"))
    (Variables|Default|SetConnect%20Enemy true)))

(event OnComponentEndOverlap(ShadowCollider2)
  (params (OverlappedComponent :type Primitive%20Component%20Object%20Reference) (OtherActor :type Actor%20Object%20Reference) (OtherComp :type Primitive%20Component%20Object%20Reference) (OtherBodyIndex :type Integer))
  (if (Math|Boolean|ORBoolean (Components|ComponentHasTag OtherComp "Enemy Shadow") (Actor|ActorHasTag OtherActor "Enemy") (Components|ComponentHasTag OtherComp "Object Shadow") (Actor|ActorHasTag OtherActor "Object"))
    (Variables|Default|SetConnect%20Enemy false)))

(event OnComponentEndOverlap(ShadowCollider3)
  (params (OverlappedComponent :type Primitive%20Component%20Object%20Reference) (OtherActor :type Actor%20Object%20Reference) (OtherComp :type Primitive%20Component%20Object%20Reference) (OtherBodyIndex :type Integer))
  (if (Math|Boolean|ORBoolean (Components|ComponentHasTag OtherComp "Enemy Shadow") (Actor|ActorHasTag OtherActor "Enemy") (Components|ComponentHasTag OtherComp "Object Shadow") (Actor|ActorHasTag OtherActor "Object"))
    (Variables|Default|SetConnect%20Enemy false)))

(event OnComponentEndOverlap(ShadowCollider1)
  (params (OverlappedComponent :type Primitive%20Component%20Object%20Reference) (OtherActor :type Actor%20Object%20Reference) (OtherComp :type Primitive%20Component%20Object%20Reference) (OtherBodyIndex :type Integer))
  (if (Math|Boolean|ORBoolean (Components|ComponentHasTag OtherComp "Enemy Shadow") (Actor|ActorHasTag OtherActor "Enemy") (Components|ComponentHasTag OtherComp "Object Shadow") (Actor|ActorHasTag OtherActor "Object"))
    (Variables|Default|SetConnect%20Enemy false)))

(event Custom|Shadow%20Collision%202
  (params (Ball :type Actor%20Object%20Reference))
  (bind _shadowcolliderroot_2 (Variables|Default|GetShadowColliderRoot%202))
  (bind _shadow_collider_2 (Variables|Default|GetShadow%20Collider%202))
  (bind _bothblocked (CallFunction|AreBothPathsBlockedtoBall Ball))
  (if _bothblocked
    (CallFunction|ResetOneShadowCollider _shadowcolliderroot_2 _shadow_collider_2)
    (else
      (CallFunction|ShadowCollisionCompute Ball _shadowcolliderroot_2 _shadow_collider_2)
      (Collision|SetCollisionEnabled _shadow_collider_2 "QueryOnly"))))

(event Custom|Shadow%20Collision%201
  (params (Ball :type Actor%20Object%20Reference))
  (bind _shadowcolliderroot_1 (Variables|Default|GetShadowColliderRoot%201))
  (bind _shadow_collider_1 (Variables|Default|GetShadow%20Collider%201))
  (bind _bothblocked (CallFunction|AreBothPathsBlockedtoBall Ball))
  (if _bothblocked
    (CallFunction|ResetOneShadowCollider _shadowcolliderroot_1 _shadow_collider_1)
    (else
      (CallFunction|ShadowCollisionCompute Ball _shadowcolliderroot_1 _shadow_collider_1)
      (Collision|SetCollisionEnabled _shadow_collider_1 "QueryOnly"))))

(event Custom|Shadow%20Collision%20Compute
  (params (Ball :type Actor%20Object%20Reference) (Target%20Root :type Scene%20Component%20Object%20Reference) (Target%20Collider :type Box%20Component%20Object%20Reference))
  (bind _returnvalue (Transformation|GetActorLocation Ball))
  (bind _shadow_point (Variables|Default|GetShadow%20Point))
  (bind _returnvalue_2 (Transformation|GetWorldLocation _shadow_point))
  (bind _returnvalue_3 (- _returnvalue_2 _returnvalue))
  (bind _returnvalue_4 (Math|Vector|Normalize _returnvalue_3))
  (bind _returnvalue_5 (* _returnvalue_4 6e+02))
  (bind _returnvalue_6 (+ _returnvalue_2 _returnvalue_5))
  (bind (_outhit _returnvalue_7) (Collision|LineTraceByChannel _returnvalue_2 _returnvalue_6 "TraceTypeQuery1" false 0 "ForDuration"))
  (bind _output_get (Variables|Default|SetShadow%20Farthest%20Location (Math|Vector|SelectVector (.Location (Collision|BreakHitResult _outhit)) (+ _returnvalue_2 (* (- _returnvalue_6 _returnvalue_2) 0.6)) _returnvalue_7)))
  (Variables|Default|SetShadow%20colision%20distance (Math|Vector|VectorLength (- _output_get (Transformation|GetWorldLocation Target%20Root))))
  (Transformation|SetWorldRotation Target%20Root (Math|Rotator|FindLookatRotation (Transformation|GetWorldLocation (Variables|Default|GetShadow%20Point)) (Variables|Default|GetShadow%20Farthest%20Location)) false false)
  (Components|Box|SetBoxExtent Target%20Collider (Math|Vector|MakeVector 3.4e+02 1e+02 35.0) true)
  (Transformation|SetRelativeLocation Target%20Collider (Math|Vector|MakeVector (/ (Math|Vector|VectorLength (- _output_get (Transformation|GetWorldLocation Target%20Root))) 1.25) 0.0 0.0) false false))

(event Custom|Check%20Overlapping%20Light%20Checker
  (for _array_element (Collision|GetOverlappingActors (Variables|Default|GetCylinder) "/Game/BluePrint/Player/BP_LightBall.BP_LightBall_C" :!class /Script/Engine.PrimitiveComponent)
    (if (== (Utilities|Array|Get(acopy) (Variables|Default|GetSlot%20Onwers)) _array_element)
      (CallFunction|ShadowCollision1 _array_element)
      (elif (== (Utilities|Array|Get(acopy) (Variables|Default|GetSlot%20Onwers) 1) _array_element)
        (CallFunction|ShadowCollision2 _array_element)
        (elif (== (Utilities|Array|Get(acopy) (Variables|Default|GetSlot%20Onwers) 2) _array_element)
          (CallFunction|ShadowCollision3 _array_element))))))

(event Custom|Shadow%20Collision%203
  (params (Ball :type Actor%20Object%20Reference))
  (bind _shadowcolliderroot_3 (Variables|Default|GetShadowColliderRoot%203))
  (bind _shadow_collider_3 (Variables|Default|GetShadow%20Collider%203))
  (bind _bothblocked (CallFunction|AreBothPathsBlockedtoBall Ball))
  (if _bothblocked
    (CallFunction|ResetOneShadowCollider _shadowcolliderroot_3 _shadow_collider_3)
    (else
      (CallFunction|ShadowCollisionCompute Ball _shadowcolliderroot_3 _shadow_collider_3)
      (Collision|SetCollisionEnabled _shadow_collider_3 "QueryOnly"))))

(event EventBeginPlay
  (Collision|SetCollisionEnabled (Variables|Default|GetShadow%20Collider%201) "NoCollision")
  (Utilities|Array|Clear (Variables|Default|GetSlot%20Onwers))
  (Utilities|Array|Add (Variables|Default|GetSlot%20Onwers) 0)
  (Utilities|Array|Add (Variables|Default|GetSlot%20Onwers) 0)
  (Utilities|Array|Add (Variables|Default|GetSlot%20Onwers) 0))

(event EventTick
  (params (DeltaSeconds :type Float%20%28single-precision%29))
  (CallFunction|CheckOverlappingLightChecker)
  (if (Variables|Default|GetConnect%20Enemy)
    _))

(fn ConstructionScript)

(fn ResetOneShadowCollider
  (params (Target%20Root :type Scene%20Component%20Object%20Reference) (Target%20Collider :type Box%20Component%20Object%20Reference))
  (Components|Box|SetBoxExtent Target%20Collider (Variables|Default|GetOrigin%20Collision%20Size) true)
  (Collision|SetCollisionEnabled Target%20Collider "NoCollision")
  (Transformation|SetRelativeLocation Target%20Collider "0, 0, 0" false false)
  (Transformation|SetWorldRotation Target%20Root "0, 0, 0" false false))

(fn IsSegmentBlocked
  (params (Start :type Vector) (End :type Vector) (Self%20Actor :type Actor%20Object%20Reference) (Light%20Ball%20Actor :type Actor%20Object%20Reference))
  (bind (_outhit _returnvalue) (Collision|LineTraceByChannel Start End "TraceTypeQuery1" false 0 "None"))
  (return (and (and _returnvalue (!= (.HitActor (Collision|BreakHitResult _outhit)) Self%20Actor)) (!= (.HitActor (Collision|BreakHitResult _outhit)) Light%20Ball%20Actor))))

(fn AreBothPathsBlockedtoBall
  (params (Light%20Ball%20Actor :type Actor%20Object%20Reference))
  (bind _returnvalue (Transformation|GetActorLocation Light%20Ball%20Actor))
  (bind _blocked (CallFunction|IsSegmentBlocked (Transformation|GetWorldLocation (Variables|Default|GetTop)) _returnvalue 0 Light%20Ball%20Actor))
  (bind _blocked_2 (CallFunction|IsSegmentBlocked (Transformation|GetWorldLocation (Variables|Default|GetButtom)) _returnvalue 0 Light%20Ball%20Actor))
  (return (and _blocked _blocked_2)))

(fn GetShadowOwner
  (return self))

(fn GetShadowRole
  (return (Utilities|Enum|LiteralenumE_ShadowRole "NewEnumerator1")))

(fn IsShadowLinkActive
  (return (Variables|Default|GetConnect%20Enemy)))