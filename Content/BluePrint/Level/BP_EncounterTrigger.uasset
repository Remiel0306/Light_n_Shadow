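; BP_EncounterTrigger is a box trigger that starts an enemy encounter when the BP_ThirdPersonCharacter overlaps it.
; It gets the BP_EnemyAIController of the referenced Hunter, then the Spotter, and calls NotifyEncounterStarted on each.
; The actor destroys itself after both notifications, making it one-shot; AlreadyTriggered is checked but never set here.
; A debug "Hello" print remains, and a TriggerCounter check is left unconnected.
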(event OnComponentBeginOverlap(Box)
  (params (OverlappedComponent :type Primitive%20Component%20Object%20Reference) (OtherActor :type Actor%20Object%20Reference) (OtherComp :type Primitive%20Component%20Object%20Reference) (OtherBodyIndex :type Integer) (bFromSweep :type Boolean) (SweepResult :type Hit%20Result%20Structure%20%28by%20ref%29))
  (Utilities|Casting|CastToBP_ThirdPersonCharacter OtherActor)
  (if (not (Variables|Default|GetAlreadyTriggered))
    (bind _asbp_enemy_aicontroller (Utilities|Casting|CastToBP_EnemyAIController (AI|GetAIController (Variables|Default|GetHunter%20Ref))))
    (Development|PrintString "Hello")
    (Default|NotifyEncounterStarted _asbp_enemy_aicontroller)
    (bind _asbp_enemy_aicontroller_2 (Utilities|Casting|CastToBP_EnemyAIController (AI|GetAIController (Variables|Default|GetSpotter%20Ref))))
    (Default|NotifyEncounterStarted _asbp_enemy_aicontroller_2)
    (Actor|DestroyActor)))

(event EventBeginPlay)

(event Collision|EventActorBeginOverlap
  (params (OtherActor :type Actor%20Object%20Reference)))

(event EventTick
  (params (DeltaSeconds :type Float%20%28single-precision%29)))

(fn ConstructionScript)