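; Spotter enemy that patrols, searches for the player and alerts a linked Hunter.
; Phase 1 walks between PointA and PointB with random halfway turns, unless the encounter has already started.
; Phase 2 moves to PointC, then periodically heads to the player's sampled location, using a grab count and random rolls to retry or return.
; StartFollow interrupts both phases, sends the Hunter's AI controller a kill request and chases the target faster on a timer.
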(event Custom|Start%20Follow
  (params (Player :type Actor%20Object%20Reference))
  (bind _hunter_ref (Variables|Default|GetHunter%20Ref))
  (if (Variables|Default|GetIsFollowing)
    (Variables|Default|SetFollow%20Target Player)
    (else
      (Development|PrintString "2")
      (Variables|Default|SetIsFollowing true)
      (Variables|Default|SetFollow%20Target Player)
      (Utilities|IsValid _hunter_ref
        (:Is%20Valid
          (bind _asbp_enemy_aicontroller (Utilities|Casting|CastToBP_EnemyAIController (AI|GetAIController _hunter_ref)))
          (Default|RequestKill _asbp_enemy_aicontroller Player)
          (Utilities|Time|SetTimerbyEvent (delegate Custom|Update%20Follow%20Move) 0.3 true)
          (Variables|Default|SetPhase2PausedForFollow true)
          (Utilities|Time|ClearandInvalidateTimerbyHandle (Variables|Default|GetPhase1TimerHandle)))))))

(event Custom|Update%20Follow%20Move
  (bind _follow_target (Variables|Default|GetFollow%20Target))
  (if (Variables|Default|GetIsFollowing)
    (Utilities|IsValid _follow_target
      (:Is%20Valid
        (Variables|/Script/Engine.CharacterMovementComponent|SetMaxWalkSpeed (Variables|Character|GetCharacterMovement) 4.2e+02)
        (AI|AIMoveTo self "0, 0, 0" _follow_target 1e+01 false)))))

(event Custom|Phase%201%20Go%20to%20A
  (bind _point_a (Variables|Default|GetPoint%20A))
  (if (not (or (Variables|Default|GetHalfWayTurn) (Variables|Default|GetIsFollowing)))
    (Development|PrintString "5")
    (Utilities|IsValid _point_a
      (:Is%20Valid
        (Utilities|FlowControl|Sequence
          (:then_0
            (AI|AIMoveTo self "0, 0, 0" _point_a 5.0 false
              (:OnSuccess
                (if (not (or (Variables|Default|GetHalfWayTurn) (Variables|Default|GetIsFollowing)))
                  (Utilities|FlowControl|Delay 0.85)
                  (CallFunction|Phase1GotoB)))
              (:OnFail
                (if (not (or (Variables|Default|GetHalfWayTurn) (Variables|Default|GetIsFollowing)))
                  (Utilities|FlowControl|Delay 0.35)
                  (CallFunction|Phase1GotoA)))))
          (:then_1
            (Utilities|Time|SetTimerbyEvent (delegate Custom|Try%20Halfway%20Turn) 0.5)))))))

(event Custom|Start%20Phase%201
  (Development|PrintString "3")
  (Variables|Default|SetPhase%202 false)
  (Variables|/Script/Engine.CharacterMovementComponent|SetMaxWalkSpeed (Variables|Character|GetCharacterMovement) 1.7e+02)
  (CallFunction|Phase1GotoB))

(event Custom|Try%20Halfway%20Turn
  (if (not (Variables|Default|GetIsFollowing))
    (if (not (Variables|Default|GetPhase%202))
      (if (< (Math|Random|RandomFloatinRange 0.0 1.0) 0.5)
        (Variables|Default|SetHalfWayTurn true)
        (Components|Movement|StopMovementImmediately (Variables|Character|GetCharacterMovement))
        (AI|AIMoveTo self "0, 0, 0" (Variables|Default|GetPoint%20B) 5.0 false
          (:OnSuccess
            (Utilities|FlowControl|Delay (Variables|Default|GetScanWaitTime))
            (Variables|Default|SetHalfWayTurn false)
            (CallFunction|Phase1GotoA))
          (:OnFail
            (Utilities|FlowControl|Delay 0.2)
            (CallFunction|Phase1GotoB)))))))

(event Custom|Phase%201%20Go%20to%20B
  (bind _point_b (Variables|Default|GetPoint%20B))
  (if (not (Variables|Default|GetIsFollowing))
    (Development|PrintString "4")
    (Utilities|IsValid _point_b
      (:Is%20Valid
        (AI|AIMoveTo self "0, 0, 0" _point_b 5.0 false
          (:OnSuccess
            (Utilities|FlowControl|Delay (Variables|Default|GetScanWaitTime))
            (CallFunction|Phase1GotoA))
          (:OnFail
            (Utilities|FlowControl|Delay 0.35)
            (CallFunction|Phase1GotoB)))))))

(event Custom|Enter%20Phase%202
  (if (not (Variables|Default|GetIsFollowing))
    (Variables|Default|SetPhase%202 true)
    (Utilities|Time|ClearandInvalidateTimerbyHandle (Variables|Default|GetPhase1TimerHandle))
    (Components|Movement|StopMovementImmediately (Variables|Character|GetCharacterMovement))
    (Utilities|IsValid (Variables|Default|GetPoint%20C)
      (:Is%20Valid
        (Variables|/Script/Engine.CharacterMovementComponent|SetMaxWalkSpeed (Variables|Character|GetCharacterMovement) 1.7e+02)
        (AI|AIMoveTo self "0, 0, 0" (Variables|Default|GetPoint%20C) 5.0 false :!label _label
          (:OnSuccess
            (CallFunction|EnterPhase2TrackLoop))
          (:OnFail
            (Utilities|FlowControl|Delay 0.5)
            (goto _label)))))))

(event Custom|Enter%20Phase%202%20Track%20Loop
  (if (not (Variables|Default|GetIsFollowing))
    (Variables|Default|SetGrabCount 0)
    (Utilities|Time|SetTimerbyEvent (delegate Custom|Phase%202%20Try%20to%20Track) (Variables|Default|GetTrackInterval) true)))

(event Custom|Phase%202%20Try%20to%20Track
  (if (Variables|Default|GetPhase%202)
    (if (not (Variables|Default|GetIsFollowing))
      (if (not (Variables|Default|GetPhase2PausedForFollow))
        (bind _output_get (Variables|Default|SetLastGrabLocation (Transformation|GetActorLocation (Game|GetPlayerCharacter 0))))
        (AI|AIMoveTo self _output_get 0 5.0 false
          (:OnSuccess
            (Utilities|FlowControl|Delay 0.2)
            (CallFunction|AfterTrackArrived))
          (:OnFail
            (Utilities|FlowControl|Delay 0.2)
            (AI|AIMoveTo self "0, 0, 0" (Variables|Default|GetPoint%20C) 5.0 false
              (:then
                (CallFunction|Phase2TrytoTrack)))))))))

(event Custom|After%20Track%20Arrived
  (if (not (Variables|Default|GetIsFollowing))
    (Variables|Default|SetGrabCount (+ (Variables|Default|GetGrabCount) 1))
    (if (>= (Variables|Default|GetGrabCount) 4)
      (Utilities|FlowControl|Delay 0.2)
      (AI|AIMoveTo self "0, 0, 0" (Variables|Default|GetPoint%20C) 5.0 false
        (:then
          (CallFunction|Phase2TrytoTrack)))
      (elif (== (Variables|Default|GetGrabCount) 1)
        (if (< (Math|Random|RandomFloatinRange 0.0 1.0) 0.4)
          _)
        (elif (== (Variables|Default|GetGrabCount) 2)
          (if (< (Math|Random|RandomFloatinRange 0.0 1.0) 0.25)
            (CallFunction|Phase2TrytoTrack :!label _label)
            (else
              (if (== (Variables|Default|GetGrabCount) 3)
                (if (< (Math|Random|RandomFloatinRange 0.0 1.0) 0.167)
                  (goto _label)
                  (elif (== (Variables|Default|GetGrabCount) 4)
                    (if (< (Math|Random|RandomFloatinRange 0.0 1.0) 0.1)
                      (goto _label)
                      (else
                        _)))))
              (AI|AIMoveTo self "0, 0, 0" (Variables|Default|GetPoint%20C) 5.0 false))))))))

(event EventBeginPlay
  (|CallParentFunction)
  (Utilities|FlowControl|Delay 0.35)
  (bind _asbp_enemy_aicontroller (Utilities|Casting|CastToBP_EnemyAIController (Pawn|GetController)))
  (Development|PrintString "1")
  (if (not (Variables|/Game/BluePrint/System/BP_EnemyAIController.BP_EnemyAIController_C|GetEncounterStarted _asbp_enemy_aicontroller))
    (CallFunction|StartPhase1)))

(event Collision|EventActorBeginOverlap
  (params (OtherActor :type Actor%20Object%20Reference)))

(event EventTick
  (params (DeltaSeconds :type Float%20%28single-precision%29))
  (|CallParentFunction DeltaSeconds) ; This node is disabled and will not be called.\nDrag off pins to build functionality.
)

(fn ConstructionScript
  (|CallParentFunction))