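; BP_LightBall is a physics light ball, tracked by the third-person character, that can be frozen mid-motion or engaged as a timed light source.
; FreezeBall toggles physics, saving and restoring velocity, hiding or showing the sphere, and re-registering as the active thrown ball on unfreeze.
; EngagetheBall freezes it, enables the light and LightChecker queries, then destroys it after a delay or on a repeat call, decrementing the character's BallCounter.
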(event Custom|Engage%20the%20Ball
  ;[0.15 0.15 0.15 0.5] Engage the Ball
  (if (Variables|Default|GetisEngaged?)
    (Actor|DestroyActor)
    (else
      (if (Variables|Default|GetisFreeze?)
        _
        (else
          (CallFunction|FreezeBall)))
      (Collision|SetCollisionEnabled (Variables|Default|GetLightChecker) "QueryOnly")
      (Rendering|SetVisibility (Variables|Default|GetPointLight) true false)
      (Variables|Default|SetisEngaged? true)
      (Utilities|FlowControl|Delay 15.0)
      (Actor|DestroyActor)))
  (bind _returnvalue (Actor|GetActorOfClass "/Game/BluePrint/BP_ThirdPersonCharacter.BP_ThirdPersonCharacter_C"))
  (Variables|/Game/BluePrint/BP_ThirdPersonCharacter.BP_ThirdPersonCharacter_C|SetBall%20Counter _returnvalue (- (Variables|/Game/BluePrint/BP_ThirdPersonCharacter.BP_ThirdPersonCharacter_C|GetBall%20Counter _returnvalue) 1)))

(event Custom|Freeze%20Ball
  (bind _sphere (Variables|Default|GetSphere))
  ;[0.15 0.15 0.15 0.5] Freeze the Ball
  (Utilities|FlowControl|FlipFlop
    (:A
      (bind _returnvalue (Physics|GetPhysicsLinearVelocity (Variables|Default|GetLightBall) "None"))
      (Variables|Default|SetSaved%20Velocity _returnvalue)
      (Physics|SetSimulatePhysics (Variables|Default|GetLightBall) false)
      (Class|PrimitiveComponent|SetAllPhysicsLinearVelocity (Variables|Default|GetLightBall) "0, 0, 0" false)
      (Variables|Default|SetisFreeze? true)
      (Utilities|FlowControl|Delay 0.2)
      (Rendering|SetVisibility _sphere false false))
    (:B
      (Physics|SetSimulatePhysics (Variables|Default|GetLightBall) true)
      (Class|PrimitiveComponent|SetAllPhysicsLinearVelocity (Variables|Default|GetLightBall) (Variables|Default|GetSaved%20Velocity) false)
      (Variables|Default|SetisFreeze? false)
      (bind _returnvalue_2 (Actor|GetActorOfClass "/Game/BluePrint/BP_ThirdPersonCharacter.BP_ThirdPersonCharacter_C"))
      (Variables|/Game/BluePrint/BP_ThirdPersonCharacter.BP_ThirdPersonCharacter_C|SetActive%20Thrown%20Ball _returnvalue_2 self)
      (Rendering|SetVisibility _sphere true false))))

(event EventBeginPlay
  (Collision|SetCollisionEnabled (Variables|Default|GetLightChecker) "NoCollision"))

(event Collision|EventActorBeginOverlap
  (params (OtherActor :type Actor%20Object%20Reference)))

(event EventTick
  (params (DeltaSeconds :type Float%20%28single-precision%29)))

(fn ConstructionScript)