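; AI controller for BP_EnemyShadowLogic enemies that wander until they perceive the player, then chase.
; Wander repeatedly moves to random reachable points at normal speed.
; Sensing the player starts a looping KeepChase timer that moves at chase speed to a point ahead of the player's velocity.
; Losing the player leaves IsChasing set; perceiving other actors resets it, but the running timer's handle is never stored, so chasing persists.
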(event OnTargetPerceptionUpdated(AIPerception)
  (params (Actor :type Actor%20Object%20Reference) (Stimulus :type AI%20Stimulus%20Structure))
  (if (== Actor (Game|GetPlayerCharacter 0))
    (if (.bSuccessfullySensed (Utilities|Struct|BreakAIStimulus Stimulus))
      (if (not (Variables|Default|GetisChasing))
        (Variables|Default|SetisChasing true)
        (Utilities|Time|SetTimerbyEvent (delegate Custom|Keep%20Chase) 0.25 true))
      (else
        (CallFunction|Wander)))
    (else
      (Variables|Default|SetisChasing false)
      (Utilities|Time|ClearandInvalidateTimerbyHandle (Variables|Default|GetChaseTimerHandle))
      (CallFunction|Wander))))

(event Custom|Wander
  (bind _enemy_ref (Variables|Default|GetEnemy%20Ref))
  (bind _wander_radious (Variables|Default|GetWander%20Radious))
  (bind _returnvalue (Transformation|GetActorLocation _enemy_ref))
  (bind (_randomlocation _returnvalue_2) (AI|Navigation|GetRandomReachablePointinRadius _returnvalue _wander_radious 0 0))
  (if (not (Variables|Default|GetisChasing))
    (if (Utilities|IsValid _enemy_ref)
      (Variables|/Script/Engine.CharacterMovementComponent|SetMaxWalkSpeed (Variables|/Script/Engine.Character|GetCharacterMovement _enemy_ref) (Variables|Default|GetNormal%20Speed))
      (if _returnvalue_2
        (AI|AIMoveTo (Variables|Default|GetEnemy%20Ref) _randomlocation 0 5e+01 false
          (:OnSuccess
            (Utilities|FlowControl|Delay 0.2)
            (CallFunction|Wander))
          (:OnFail
            (Utilities|FlowControl|Delay 0.5)
            (CallFunction|Wander)))))))

(event Custom|Keep%20Chase
  (bind _returnvalue (Game|GetPlayerCharacter 0))
  (bind _enemy_ref (Variables|Default|GetEnemy%20Ref))
  (Variables|/Script/Engine.CharacterMovementComponent|SetMaxWalkSpeed (Variables|/Script/Engine.Character|GetCharacterMovement _enemy_ref) (Variables|Default|GetChase%20Speed))
  (AI|AIMoveTo _enemy_ref (+ (Transformation|GetActorLocation _returnvalue) (* (Math|Vector|Normalize (Transformation|GetVelocity _returnvalue) 1.0) 2.5e+02)) 0 1e+01 false
    (:OnSuccess
      (if (not true)
        (Variables|Default|SetisChasing true)
        (bind _returnvalue_2 (Utilities|Time|SetTimerbyEvent (delegate Custom|Keep%20Chase) 0.25 true))
        (Variables|Default|SetChaseTimerHandle _returnvalue_2)))))

(event EventBeginPlay
  (Components|Activation|SetActive (Variables|Default|GetAIPerception) true false)
  (Class|AIPerceptionComponent|RequestStimuliListenerUpdate (Variables|Default|GetAIPerception))
  (bind _asbp_enemy_shadow_logic (Utilities|Casting|CastToBP_EnemyShadowLogic (Pawn|GetControlledPawn)))
  (Variables|Default|SetEnemy%20Ref _asbp_enemy_shadow_logic)
  (CallFunction|Wander))

(fn ConstructionScript)